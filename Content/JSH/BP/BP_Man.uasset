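; BP_Man is an actor with a zoomable, rotatable spring-arm camera that removes itself on a signal from the player.
; Each tick it casts the player character to BP_Topdown and destroys itself when that character's JSHFSM DelMan flag is set.
; ZoomCam and RotateCam ease input values with delta-time lerps to drive clamped arm length and yaw, though nothing in these graphs calls them.
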(event `self.ReceiveTick`
  (params (DeltaSeconds :type "Float (single-precision)"))
  (bind _asbp_topdown (cast `/Game/JSH/BP/BP_Topdown` (`GameplayStatics.GetPlayerCharacter` 0)))
  (if (`JSH_FSM.DelMan` (`/Game/JSH/BP/BP_Topdown.JSH_FSM` _asbp_topdown))
    (`/Engine/EditorBlueprintResources/StandardMacros.IsValid` self
      (:`Is Valid`
        (`self.K2_DestroyActor`)))))

(fn `RotateCam`
  (bind _output_get (set `self.RotationRate` (`KismetMathLibrary.Lerp` (`self.RotationRate`) (* (`|GetInputActionValue`) 1.0) (* (`GameplayStatics.GetWorldDeltaSeconds`) 5.0))))
  (`SceneComponent.K2_AddRelativeRotation` (`self.SpringArm`) (`KismetMathLibrary.MakeRotator` 0.0 0.0 _output_get) false false))

(fn `UserConstructionScript`)

(fn `ZoomCam`
  (bind _springarm (`self.SpringArm`))
  (bind _output_get (set `self.ZoomRotate` (`KismetMathLibrary.Lerp` (`self.ZoomRotate`) (* (`|GetInputActionValue`) 100.0) (* (`GameplayStatics.GetWorldDeltaSeconds`) 5.0))))
  (set `SpringArmComponent.TargetArmLength` (`KismetMathLibrary.FClamp` (+ (`SpringArmComponent.TargetArmLength` _springarm) _output_get) 500.0 10000.0) _springarm))