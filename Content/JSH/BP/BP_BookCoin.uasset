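; BP_BookCoin is an actor that shows a rising, spinning coin when the top-down player's Coin flag is set.
; Tick polls that flag on BP_Topdown, then reveals the coin, increments its BookCoin counter and nudges height and yaw every frame.
; Steps add DeltaSeconds to fixed amounts, so motion depends on frame rate.
; A half-second Delay then clears the player's flag and destroys the actor.
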(event `self.ReceiveBeginPlay`)

(event `self.ReceiveTick`
  (params (DeltaSeconds :type "Float (single-precision)"))
  (bind (_returnvalue_x _returnvalue_y _returnvalue_z) (`KismetMathLibrary.BreakVector` (`SceneComponent.GetSocketLocation` (`self.Coin`) "None")))
  (bind (_returnvalue_roll _returnvalue_pitch _returnvalue_yaw) (`KismetMathLibrary.BreakRotator` (`SceneComponent.GetSocketRotation` (`self.Coin`) "None")))
  (bind _asbp_topdown (cast `/Game/JSH/BP/BP_Topdown` (`GameplayStatics.GetPlayerCharacter` 0)))
  (if (`/Game/JSH/BP/BP_Topdown.Coin++` _asbp_topdown)
    (`SceneComponent.SetVisibility` (`self.Coin`) true false)
    (set `self.Book Coin` (`KismetMathLibrary.FTrunc` (+ (`self.Book Coin`) 1.0)))
    (`SceneComponent.K2_SetWorldLocation` (`self.Coin`) (`KismetMathLibrary.MakeVector` _returnvalue_x _returnvalue_y (+ _returnvalue_z (+ DeltaSeconds 2.0))) false false)
    (`SceneComponent.K2_SetWorldRotation` (`self.Coin`) (`KismetMathLibrary.MakeRotator` _returnvalue_roll _returnvalue_pitch (+ _returnvalue_yaw (+ DeltaSeconds 10.0))) false false)
    (`KismetSystemLibrary.Delay` 0.5)
    (set `/Game/JSH/BP/BP_Topdown.Coin++` false _asbp_topdown)
    (`self.K2_DestroyActor`)))

(event `Key|MiddleMouseButton`
  (params (Key :type "Key Structure")))

(fn `UserConstructionScript`)