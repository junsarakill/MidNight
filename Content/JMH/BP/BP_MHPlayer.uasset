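; BP_MHPlayer is a player Blueprint that triggers fairy-tale actions: scattering breadcrumbs and eating the candy house.
; BeginPlay enables input, and key 1 calls HandlePlayerActions.
; That function switches on a constant 1, so it always calls DropBread on MHDrop.
; The unreached case 2 would call ScaleDownSnack on the MH_ScaleDownComponent of every BP_Snack in the level.
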(event `Key|One`
  (params (Key :type "Key Structure"))
  ;[1 1 1] 1~5
  (:`Pressed`
    (`self.HandlePlayerActions`)))

(event `self.ReceiveBeginPlay`
  (`parent.ReceiveBeginPlay`)
  (`self.EnableInput` (`GameplayStatics.GetPlayerController` 0) null))

(fn `HandlePlayerActions`
  (switch `int` 1
    (:`1`
      ;[1 1 1] 빵조각뿌리기
      (`MH_DropComponent.DropBread` (`self.MH_Drop`)))
    (:`2`
      ;[1 1 1] 과자집먹기
      (bind _outactors (`GameplayStatics.GetAllActorsOfClass` "/Game/JMH/BP/BP_Snack.BP_Snack_C"))
      (for _array_element _outactors
        (`MH_ScaleDownComponent.ScaleDownSnack` (`self.GetComponentByClass` _array_element "/Script/MidNight.MH_ScaleDownComponent"))))))

(fn `UserConstructionScript`
  (`parent.UserConstructionScript`))