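; BP_MH_GretelPlayer is a Gretel player Blueprint that triggers fairy-tale scene actions from the 2 key.
; A switch on a fixed value of 1 makes the key drop bread and move the player through MHDrop.
; Its other, currently unreachable cases find all snack, witch hand or Gretel hand actors and call their components to shrink snacks, move hands or rotate hands for the potion.
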(event `Key|Two`
  (params (Key :type "Key Structure"))
  (bind _mh_drop (`self.MH_Drop`))
  (:`Pressed`
    (switch `int` 1
      (:`1`
        (`|ExecutionSequence`
          (:`then_0`
            (`MH_DropComponent.DropBread` _mh_drop))
          (:`then_1`
            (`MH_DropComponent.MovePlayer` _mh_drop))))
      (:`2`
        ;[1 1 1] 과자집먹기
        (bind _outactors (`GameplayStatics.GetAllActorsOfClass` "/Game/JMH/BP/BP_Snack.BP_Snack_C"))
        (for _array_element _outactors
          (`MH_ScaleDownComponent.ScaleDownSnack` (`self.GetComponentByClass` _array_element "/Script/MidNight.MH_ScaleDownComponent"))))
      (:`4`
        ;[1 1 1] 과자집먹기
        (bind _outactors_2 (`GameplayStatics.GetAllActorsOfClass` "/Game/JMH/BP/BP_WitchHand.BP_WitchHand_C"))
        (for _array_element_2 _outactors_2
          (`MH_HandMoveComponent.MoveHandToTarget` (`self.GetComponentByClass` _array_element_2 "/Script/MidNight.MH_HandMoveComponent"))))
      (:`5`
        ;[1 1 1] 물약
        (bind _outactors_3 (`GameplayStatics.GetAllActorsOfClass` "/Game/JMH/BP/BP_GretelHand.BP_GretelHand_C"))
        (for _array_element_3 _outactors_3
          (`MH_RotationHandComponent.RotateHand` (`self.GetComponentByClass` _array_element_3 "/Script/MidNight.MH_RotationHandComponent") 1))))))

(fn `UserConstructionScript`)